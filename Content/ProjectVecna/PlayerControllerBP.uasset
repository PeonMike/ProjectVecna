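; Player controller for ProjectVecna that sets up the player's HUD and provides a manual save key.
; On BeginPlay, only the local controller creates the Main_HUD widget, adds it to the viewport and switches input to game-only.
; Pressing L casts the game mode to PVGameModeBase, calls WriteSaveGame and prints a confirmation message.
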(event EventBeginPlay
  (if (Pawn|IsLocalController)
    (bind _returnvalue (UserInterface|CreateWidget "/Game/ProjectVecna/UI/Main_HUD.Main_HUD_C"))
    (UserInterface|Viewport|AddtoViewport _returnvalue 0)
    (Input|SetInputModeGameOnly self)))

(event Input|KeyboardEvents|L
  (params (Key :type Key%20Structure :default "None"))
  (:Pressed
    (bind _aspvgame_mode_base (Utilities|Casting|CastToPVGameModeBase (Game|GetGameMode)))
    (Class|PVGameModeBase|WriteSaveGame _aspvgame_mode_base)
    (Development|PrintString "SAVE WRITEN")))

(fn ConstructionScript)